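; BP_Zombie is an enemy that chases the player, plays an attack montage on arrival, then resumes pursuit.
; AIMoveTo drives the chase loop, and seeing a pawn through PawnSensing raises its walk speed.
; Point damage lowers health, playing a hit reaction or triggering death.
; Death picks a headshot or bodyshot montage from the player character's WichShot, then relaxes capsule and mesh collision.
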(event `self.PawnSensing.OnSeePawn`
  (params (Pawn :type "Pawn Object Reference"))
  (set `CharacterMovementComponent.MaxWalkSpeed` 360.0 (`self.CharacterMovement`)))

(event `self.ReceiveBeginPlay`
  (`self.RunToPlayer`))

(event `RunToPlayer`
  (if (not (`self.IsDead?`))
    (`|AIMoveTo` self (0.0 0.0 0.0) (`GameplayStatics.GetPlayerPawn` 0) 40.0
      (:`OnSuccess`
        (`self.Attack`))
      (:`OnFail`
        (`self.RunToPlayer`)))))

(event `Attack`
  (`|PlayMontage` (`self.Mesh`) "/Game/_Main/Zombie/Animations/zombie_attack_Montage.zombie_attack_Montage"
    (:`OnCompleted`
      (`self.RunToPlayer`))))

(event `self.ReceivePointDamage`
  (params (Damage :type "Float (single-precision)") (DamageType :type "DamageType Object Reference") (HitLocation :type "Vector Structure") (HitNormal :type "Vector Structure") (HitComponent :type "PrimitiveComponent Object Reference") (BoneName :type Name) (ShotFromDirection :type "Vector Structure") (InstigatedBy :type "Controller Object Reference") (DamageCauser :type "Actor Object Reference") (HitInfo :type "HitResult Structure (by ref)"))
  (bind _health (`self.Health`))
  (if (`self.IsDead?`)
    _
    (elif (<= _health 0.0)
      (`self.Death`)
      (else
        (bind _output_get (set `self.Health` (- _health Damage)))
        (`KismetSystemLibrary.PrintString` (`KismetStringLibrary.Conv_DoubleToString` _output_get))
        (if (<= _output_get 0.0)
          (`self.Death`)
          (else
            (`|PlayMontage` (`self.Mesh`) "/Game/_Main/Zombie/Animations/Zombie_Reaction_Hit_Montage.Zombie_Reaction_Hit_Montage")))))))

(event `Death`
  (bind _mesh (`self.Mesh`))
  (set `self.IsDead?` true)
  (`MovementComponent.StopMovementImmediately` (`self.CharacterMovement`))
  (bind _asbp_first_person_character (cast `/Game/_Main/Character/Blueprint/BP_FirstPersonCharacter` (`GameplayStatics.GetPlayerPawn` 0)))
  (switch `int` (`/Game/_Main/Character/Blueprint/BP_FirstPersonCharacter.WichShot` _asbp_first_person_character)
    (:`0`
      (`|PlayMontage` _mesh "/Game/_Main/Zombie/Animations/zombie_death_Montage.zombie_death_Montage"
        (:`then`
          (`KismetSystemLibrary.PrintString` "HeadShot"))))
    (:`1`
      (`|PlayMontage` _mesh "/Game/_Main/Zombie/Animations/zombie_dying_Montage.zombie_dying_Montage"
        (:`then`
          (`KismetSystemLibrary.PrintString` "BodyShot")))))
  (`PrimitiveComponent.SetCollisionResponseToChannel` (`self.CapsuleComponent`) "ECC_Pawn" "ECR_Overlap")
  (`PrimitiveComponent.SetCollisionEnabled` (`self.Mesh`) "NoCollision"))

(fn `UserConstructionScript`)